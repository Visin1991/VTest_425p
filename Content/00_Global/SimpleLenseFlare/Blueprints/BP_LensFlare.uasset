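; Actor that fakes a screen-space lens flare at its world location using UMG widgets.
; BeginPlay creates a light-source widget and one lens widget per LensTypes entry, configuring material, gradient, size and index.
; Tick traces to the camera, switching visibility on both widget types for occlusion.
; It also centers the source widget on the DPI-corrected projected position, scaling intensity by distance from screen center; Destroyed removes all widgets.
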(event `self.ReceiveDestroyed`
  (`Widget.RemoveFromParent` (`self.WBP_LensFlare_LightSource`))
  (for _array_element (`self.WBP_LensFlare_Lens`)
    (if (`KismetSystemLibrary.IsValid` _array_element)
      (`Widget.RemoveFromParent` _array_element))))

(event `self.ReceiveBeginPlay`
  (bind _returnvalue (`self.K2_GetActorLocation`))
  ;[1 1 1] Create Light Source UI
  (bind _returnvalue_2 (`|CreateWidget` "/Game/00_Global/SimpleLenseFlare/Blueprints/WBP_LensFlare_LightSource.WBP_LensFlare_LightSource_C"))
  (if (`KismetSystemLibrary.IsValid` _returnvalue_2)
    (bind _output_get (set `self.WBP_LensFlare_LightSource` _returnvalue_2))
    (`UserWidget.AddToViewport` _output_get 0)
    (`/Game/00_Global/SimpleLenseFlare/Blueprints/WBP_LensFlare_LightSource.SetLightSourcePos` _output_get _returnvalue)
    (set `self.LensIndex` 0)
    (for _array_element (`self.LensTypes`)
      (bind _returnvalue_3 (`|CreateWidget` "/Game/00_Global/SimpleLenseFlare/Blueprints/WBP_LensFlare_Lens.WBP_LensFlare_Lens_C"))
      (if (`KismetSystemLibrary.IsValid` _returnvalue_3)
        (`KismetArrayLibrary.Array_AddUnique` (`self.WBP_LensFlare_Lens`) _returnvalue_3)
        (`/Game/00_Global/SimpleLenseFlare/Blueprints/WBP_LensFlare_Lens.SetMaterial` _returnvalue_3 (break `/Game/00_Global/SimpleLenseFlare/Blueprints/LensTypes` _array_element) (`KismetMathLibrary.Conv_IntToDouble` (`.GradientIndex_12_06484D2640538CAB5DD179AEED311F28` (break `/Game/00_Global/SimpleLenseFlare/Blueprints/LensTypes` _array_element))))
        (`UserWidget.AddToViewport` _returnvalue_3 0)
        (`/Game/00_Global/SimpleLenseFlare/Blueprints/WBP_LensFlare_Lens.SetImageSize` _returnvalue_3 (`.Size_9_6AB8C55D4A82B892BC5D058DA43A5A2C` (break `/Game/00_Global/SimpleLenseFlare/Blueprints/LensTypes` _array_element)))
        (bind _output_get_2 (set `self.LensIndex` (+ (`self.LensIndex`) 1)))
        (`/Game/00_Global/SimpleLenseFlare/Blueprints/WBP_LensFlare_Lens.SetLensIndex` _returnvalue_3 _output_get_2)
        (set `/Game/00_Global/SimpleLenseFlare/Blueprints/WBP_LensFlare_Lens.LightSourcePos` _returnvalue _returnvalue_3)
        (`/Game/00_Global/SimpleLenseFlare/Blueprints/WBP_LensFlare_Lens.SetToLightStepLength` _returnvalue_3 (`self.ToLightStepLenth`))))))

(event `self.ReceiveActorBeginOverlap`
  (params (OtherActor :type "Actor Object Reference")))

(event `self.ReceiveTick`
  (params (DeltaSeconds :type "Float (single-precision)"))
  (bind _wbp_lensflare_lightsource (`self.WBP_LensFlare_LightSource`))
  (bind (_outhit _returnvalue) (`KismetSystemLibrary.LineTraceSingle` (`self.K2_GetActorLocation`) (`PlayerCameraManager.GetCameraLocation` (`PlayerController.PlayerCameraManager` (`GameplayStatics.GetPlayerController` 0))) "TraceTypeQuery1"))
  (`|ExecutionSequence`
    (:`then_0`
      (if _returnvalue
        (set `self.VisibilityIntensity` 0.0)
        (else
          (set `self.VisibilityIntensity` 1.0))))
    (:`then_1`
      ;[1 1 1] Set Visibility For Lens
      (`self.CalculateLightSource`)
      (for _array_element (`self.WBP_LensFlare_Lens`)
        (if (`KismetSystemLibrary.IsValid` _array_element)
          (set `/Game/00_Global/SimpleLenseFlare/Blueprints/WBP_LensFlare_Lens.VisibilityIntensity` (`self.VisibilityIntensity`) _array_element))))
    (:`then_2`
      (if (`KismetSystemLibrary.IsValid` _wbp_lensflare_lightsource)
        (`/Game/00_Global/SimpleLenseFlare/Blueprints/WBP_LensFlare_LightSource.SetVisibilityIntensity` _wbp_lensflare_lightsource (`self.VisibilityIntensity`))))))

(fn `CalculateLightSource`
  (bind _returnvalue (`WidgetLayoutLibrary.GetViewportSize`))
  (bind _returnvalue_2 (`WidgetLayoutLibrary.GetViewportScale`))
  (bind _returnvalue_3 (/ (`GameplayStatics.ProjectWorldToScreen` (`GameplayStatics.GetPlayerController` 0) (`self.K2_GetActorLocation`)) _returnvalue_2))
  ;[1 1 1] Move Image Center ; Todo : Need to cache the size Instead of call it every frame
  (bind _imagesize (`/Game/00_Global/SimpleLenseFlare/Blueprints/WBP_LensFlare_LightSource.GetImageSize` (`self.WBP_LensFlare_LightSource`)))
  (`UserWidget.SetPositionInViewport` (`self.WBP_LensFlare_LightSource`) (- _returnvalue_3 (* _imagesize 0.5)) false)
  (`/Game/00_Global/SimpleLenseFlare/Blueprints/WBP_LensFlare_LightSource.SetLightIntensity` (`self.WBP_LensFlare_LightSource`) (`KismetMathLibrary.FClamp` (- 1.0 (/ (`KismetMathLibrary.VSize2D` (- (/ (* _returnvalue 0.5) _returnvalue_2) _returnvalue_3)) (`.Y` (`KismetMathLibrary.BreakVector2D` _returnvalue)))))))

(fn `UserConstructionScript`)